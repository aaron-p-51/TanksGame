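; Floating text spawner that shows damage numbers and damage modifier labels on an instigating player's screen.
; SpawnFloatingText requires a valid PlayerController instigator, offsets the actor location, then looks up damage type and modifier in separate config maps.
; Each match supplies widget class, color, font, pop-up and distance-scaling flags; damage is truncated to an integer.
; CreateFloatingTextWidget creates the widget, adds it to the viewport and activates it at that world position.
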(fn ConstructionScript)

(fn SpawnFloatingText
  (params (Instigator :type Controller%20Object%20Reference) (ActorLocation :type Vector) (SpawnOffset :type Vector) (DamageType :type EDamageTypes%20Enum :default "NewEnumerator0") (DamageTaken :type Float%20%28single-precision%29) (DamageModifier :type EDamageModifiers%20Enum :default "NewEnumerator0"))
  (bind _damagetextsconfig (Variables|Config|GetDamageTextsConfig))
  (bind _damagemodifiertextsconfig (Variables|Config|GetDamageModifierTextsConfig))
  (bind (_value _returnvalue) (Utilities|Map|Find _damagetextsconfig DamageType))
  (bind (_value_2 _returnvalue_2) (Utilities|Map|Find _damagemodifiertextsconfig DamageModifier))
  ;[0 1 1 0.5] Spawns Floating Texts for Damage/Damage Modifiers
  (Utilities|IsValid Instigator
    (:Is%20Valid
      (bind _asplayer_controller (Utilities|Casting|CastToPlayerController Instigator))
      (LocalVariables|SetLocal_SpawnWorldPosition (+ ActorLocation SpawnOffset))
      ;;[1 1 1] Damage Text Widget Creation
      (if (Utilities|Enum|NotEqual(Enum) DamageType "NewEnumerator0")
        (if _returnvalue
          (bind _output_get (LocalVariables|SetLocal_DamageWidgetConfig _value))
          (CallFunction|CreateFloatingTextWidget (.widgetclass _output_get) _asplayer_controller (.busepopupeffect _output_get) (.busedistancebasedscaling _output_get) (LocalVariables|GetLocal_SpawnWorldPosition) (.color _output_get) (.fontinfo _output_get) (Utilities|Text|ToText(Integer) (Math|Float|Truncate DamageTaken)))))
      ;;[1 1 1] Damage Modifier Text Widget Creation
      (if (Utilities|Enum|NotEqual(Enum) DamageModifier "NewEnumerator0")
        (if _returnvalue_2
          (bind _output_get_2 (LocalVariables|SetLocal_DamageModifierWidgetConfig _value_2))
          (CallFunction|CreateFloatingTextWidget (.widgetclass _output_get_2) _asplayer_controller (.busepopupeffect _output_get_2) (.busedistancebasedscaling _output_get_2) (LocalVariables|GetLocal_SpawnWorldPosition) (.color _output_get_2) (.fontinfo _output_get_2) (.text _output_get_2)))))))

(fn CreateFloatingTextWidget
  (params (Class :type User%20Widget%20Class%20Reference) (OwningPlayer :type Player%20Controller%20Object%20Reference) (bUsePopUpEffect :type Boolean) (bHasDistanceBasedScaling :type Boolean) (WorldPosition :type Vector) (TextColor :type Linear%20Color%20Structure) (FontInfo :type Slate%20Font%20Info%20Structure) (Text :type Text))
  ;[0 1 1 0.5] Creates & Initializes the Floating Text Widget
  (bind _returnvalue (UserInterface|CreateWidget Class OwningPlayer))
  (UserInterface|Viewport|AddtoViewport _returnvalue 0)
  (Class|BPIFloatingTextControl|ActivateFloatingText(Message) _returnvalue WorldPosition bUsePopUpEffect bHasDistanceBasedScaling TextColor FontInfo Text) ; Widget Initialization
)