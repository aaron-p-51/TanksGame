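; Player-controlled tank pawn for a simple demo game, with WASD driving, mouse aiming and firing.
; The mouse rotates the spring arm, which sets turret yaw and the pitch of spawned team-tagged bullets.
; Enemy bullets overlapping the hit box reduce LifeStat.
; At zero, it spawns wheel, body and tower physics proxies, whose transforms Tick feeds into the AnimBlueprint so the skeletal mesh falls apart.
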(event OnComponentBeginOverlap(Box)
  (params (OverlappedComponent :type Primitive%20Component%20Object%20Reference) (OtherActor :type Actor%20Object%20Reference) (OtherComp :type Primitive%20Component%20Object%20Reference) (OtherBodyIndex :type Integer) (bFromSweep :type Boolean) (SweepResult :type Hit%20Result%20Structure%20%28by%20ref%29))
  ;[1 1 1] detect hit
  (bind _asbp_bullet (Utilities|Casting|CastToBP_Bullet OtherActor))
  (if (Utilities|Enum|NotEqual(Enum) (Variables|/Game/SCTanks/DemoSimpleGame/BluePrints/BP_Bullet.BP_Bullet_C|GetTeam _asbp_bullet) (Variables|Default|GetTeam))
    (Audio|PlaySoundatLocation "/Game/SCTanks/DemoSimpleGame/Sounds/shellExplosive.shellExplosive" (Transformation|GetActorLocation) "0, 0, 0" 0.4 1.0 0.0 "/Game/SCTanks/DemoSimpleGame/Sounds/NewSoundAttenuation.NewSoundAttenuation" 0 0)
    (Actor|DestroyActor OtherActor)
    (if (> (Variables|Default|GetLifeStat) 0)
      (Variables|Default|SetLifeStat (- (Variables|Default|GetLifeStat) 10))
      (if (<= (Variables|Default|GetLifeStat) 0)
        (Components|Activation|SetActive (Variables|Default|GetAudio_Idle) false false)
        (Physics|SetSimulatePhysics (Variables|Character|GetMesh) false)
        (|createPartsforPhisicsDie)))))

(event EventTick
  (params (DeltaSeconds :type Float%20%28single-precision%29))
  (if (<= (Variables|Default|GetLifeStat) 0)
    ;[1 1 1] Die
    (bind _asanim_blueprint_tank_player (Utilities|Casting|CastToAnimBlueprint_TankPlayer (Components|SkeletalMesh|GetAnimInstance (Variables|Character|GetMesh))))
    (Utilities|IsValid (Utilities|Array|Get(acopy) (Variables|Default|GetPartsOfTankForDie))
      (:Is%20Valid
        (Variables|/Game/SCTanks/DemoSimpleGame/BluePrints/AnimBlueprint_TankPlayer.AnimBlueprint_TankPlayer_C|Setst_Blend _asanim_blueprint_tank_player 1.0)
        (for (_ _array_index) (Variables|/Game/SCTanks/DemoSimpleGame/BluePrints/AnimBlueprint_TankPlayer.AnimBlueprint_TankPlayer_C|Getst_setPosRot _asanim_blueprint_tank_player)
          (Utilities|Array|SetArrayElem (Variables|/Game/SCTanks/DemoSimpleGame/BluePrints/AnimBlueprint_TankPlayer.AnimBlueprint_TankPlayer_C|Getst_setPosRot _asanim_blueprint_tank_player) _array_index (Transformation|GetActorTransform (Utilities|Array|Get(acopy) (Variables|Default|GetPartsOfTankForDie) _array_index))))))
    (else
      ;[1 1 1] Sound of Engine Tank
      (Audio|Components|Audio|SetPitchMultiplier (Variables|Default|GetAudio_Idle) (+ (Math|Float|Clamp(Float) (/ (Class|WheeledVehicleMovementComponent|GetEngineRotationSpeed (Variables|Default|GetVehicleMovement)) 8e+02)) 1.0)))))

(event Input|MouseEvents|MouseX
  (params (AxisValue :type Float%20%28single-precision%29))
  (bind _springarm (Variables|Default|GetSpringArm))
  (bind _tower (Variables|Default|GetTower))
  ;[1 1 1] turn tower and camera
  (Transformation|AddRelativeRotation _springarm (Math|Rotator|MakeRotator 0.0 0.0 AxisValue) false false)
  (if (> (Variables|Default|GetLifeStat) 0)
    (Transformation|SetRelativeRotation _tower (Math|Rotator|MakeRotator 0.0 0.0 (+ (* (.yaw (Transformation|GetActorRotation (Components|GetOwner _springarm))) -1.0) (.yaw (Class|SpringArmComponent|GetTargetRotation _springarm)))) false false)
    (else
      (Transformation|SetRelativeRotation _tower (Math|Rotator|MakeRotator 0.0 0.0 0.0) false false))))

(event Input|MouseEvents|MouseY
  (params (AxisValue :type Float%20%28single-precision%29))
  ;[1 1 1] turn tower and camera
  (Transformation|AddRelativeRotation (Variables|Default|GetSpringArm) (Math|Rotator|MakeRotator 0.0 AxisValue 0.0) false false))

(event Input|MouseEvents|LeftMouseButton
  (params (Key :type Key%20Structure))
  (bind _bulletout (Variables|Default|GetBulletOut))
  (bind _returnvalue (Transformation|GetWorldLocation _bulletout))
  (bind _returnvalue_2 (Transformation|GetWorldRotation _bulletout))
  ;[1 1 1] shot
  (:Pressed
    (if (> (Variables|Default|GetLifeStat) 0)
      (Components|Animation|PlayAnimation (Variables|Default|GetTower) "/Game/SCTanks/DemoSimpleGame/Meshes/Tank_T34_Tower_Fire_Anim.Tank_T34_Tower_Fire_Anim" false)
      (bind _returnvalue_3 (Game|SpawnActorfromClass "/Game/SCTanks/DemoSimpleGame/BluePrints/BP_Bullet.BP_Bullet_C" (Math|Transform|MakeTransform _returnvalue (Math|Rotator|MakeRotator (.roll _returnvalue_2) (+ (.Pitch (Math|Rotator|BreakRotator (Transformation|GetWorldRotation (Variables|Default|GetSpringArm)))) 25.0) (.yaw _returnvalue_2)) "0.500000,0.300000,0.300000") "Undefined" 0 0))
      (Variables|/Game/SCTanks/DemoSimpleGame/BluePrints/BP_Bullet.BP_Bullet_C|SetTeam _returnvalue_3 (Variables|Default|GetTeam))
      (Audio|PlaySoundatLocation "/Game/SCTanks/DemoSimpleGame/Sounds/tankShot.tankShot" _returnvalue "0, 0, 0" 1.5 1.0 0.0 "/Game/SCTanks/DemoSimpleGame/Sounds/NewSoundAttenuation.NewSoundAttenuation" 0 0))))

(event Input|KeyboardEvents|A
  (params (Key :type Key%20Structure))
  (bind _vehiclemovement (Variables|Default|GetVehicleMovement))
  ;[1 1 1] turn left-right
  (:Pressed
    (Class|WheeledVehicleMovementComponent|SetSteeringInput _vehiclemovement -1.0))
  (:Released
    (Class|WheeledVehicleMovementComponent|SetSteeringInput _vehiclemovement 0.0)))

(event Input|KeyboardEvents|S
  (params (Key :type Key%20Structure))
  (bind _vehiclemovement (Variables|Default|GetVehicleMovement))
  ;[1 1 1] move forward-back
  (:Pressed
    (Class|WheeledVehicleMovementComponent|SetThrottleInput _vehiclemovement -1.0))
  (:Released
    (Class|WheeledVehicleMovementComponent|SetThrottleInput _vehiclemovement 0.0)))

(event Input|KeyboardEvents|D
  (params (Key :type Key%20Structure))
  (bind _vehiclemovement (Variables|Default|GetVehicleMovement))
  ;[1 1 1] turn left-right
  (:Pressed
    (Class|WheeledVehicleMovementComponent|SetSteeringInput _vehiclemovement 1.0))
  (:Released
    (Class|WheeledVehicleMovementComponent|SetSteeringInput _vehiclemovement 0.0)))

(event Input|KeyboardEvents|W
  (params (Key :type Key%20Structure))
  (bind _vehiclemovement (Variables|Default|GetVehicleMovement))
  ;[1 1 1] move forward-back
  (:Pressed
    (Class|WheeledVehicleMovementComponent|SetThrottleInput _vehiclemovement 1.0))
  (:Released
    (Class|WheeledVehicleMovementComponent|SetThrottleInput _vehiclemovement 0.0)))

(fn ConstructionScript)