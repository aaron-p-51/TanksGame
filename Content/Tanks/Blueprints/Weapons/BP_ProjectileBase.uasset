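; Base projectile Blueprint for the tank weapons that handles the visual wind-down of a projectile before it is destroyed.
; FinishDestroyProjectile runs a timeline that shrinks the trail effect component toward zero scale, then destroys the actor after a short delay.
; All axes follow the current world Z scale, re-read each update, so a non-uniform scale only prints a warning before fading.
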(event EventFinishDestroyProjectile
  (bind _traileffectcomp (Variables|Default|GetTrailEffectComp))
  (bind _returnvalue (Transformation|GetWorldScale _traileffectcomp))
  ;[1 1 1] Fade out TrailEffectComp
  ;;[0.779 1 0.3783] Check if world scale for TrailEffectComp is equal in all direction, if not alert but still continue
  (if (and (== (.x _returnvalue) (.y _returnvalue)) (== (.y _returnvalue) (.z _returnvalue)))
    ;;[1 0.5523 0.2764] Scale TrailEffectComp size to 0 before destroying
    (bind _fadeout (Timeline|FadeoutTrailEffects Play)
      (:Update
        (Transformation|SetWorldScale3D (Variables|Default|GetTrailEffectComp) (Math|Vector|MakeVector (Math|Float|MapRangeClamped _fadeout 1.0 0.0 (.z _returnvalue) 0.0) (Math|Float|MapRangeClamped _fadeout 1.0 0.0 (.z _returnvalue) 0.0) (Math|Float|MapRangeClamped _fadeout 1.0 0.0 (.z _returnvalue) 0.0))))
      (:Finished
        ;[1 1 1] Delay for stability then destroy
        (Utilities|FlowControl|Delay 0.2)
        (Actor|DestroyActor)))
    (else
      (Development|PrintString (Utilities|String|Append (Class|KismetSystemLibrary|GetGameName) " has unequal world scale! Unevel Fadeout trail effects"))
      (Timeline|FadeoutTrailEffects Play))))

(fn ConstructionScript)