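; BP_BasePlayerController is the base player controller that shows floating damage numbers in the tank game.
; On BeginPlay it caches the first BP_FloatingTextSpawner actor found in the level.
; Its SpawnDamageDisplayWidget event asks that spawner to show the absolute damage above a given location, with a small random horizontal offset so numbers scatter.
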(event EventBeginPlay
  (bind _outactors (Actor|GetAllActorsOfClass "/Game/FloatingDamageTexts/Blueprints/Core/BP_FloatingTextSpawner.BP_FloatingTextSpawner_C"))
  (Utilities|IsValid (Utilities|Array|Get(acopy) _outactors)
    (:Is%20Valid
      (Variables|Default|SetFloating%20Text%20Spawner (Utilities|Array|Get(acopy) _outactors)))))

(event EventSpawnDamageDisplayWidget
  (params (DisplayLocation :type Vector%20Net%20Quantize%20Structure) (Damage :type Float%20%28single-precision%29))
  (bind _floating_text_spawner (Variables|Default|GetFloating%20Text%20Spawner))
  (Utilities|IsValid _floating_text_spawner
    (:Is%20Valid
      (Default|SpawnFloatingText _floating_text_spawner self DisplayLocation (Math|Vector|MakeVector (Math|Random|RandomFloatinRange -2e+01 2e+01) (Math|Random|RandomFloatinRange -2e+01 2e+01) 1.5e+02) "NewEnumerator1" (Math|Float|Absolute(Float) Damage) "NewEnumerator0"))))

(fn ConstructionScript)