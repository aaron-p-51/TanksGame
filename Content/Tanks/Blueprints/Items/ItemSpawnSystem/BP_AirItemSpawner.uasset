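; BP_AirItemSpawner is an air item-drop spawner actor for the tank game; its graph contains only debug visualization, with no spawning logic.
; SetDebugLocations records each drop zone's position and a matching air-drop point directly above or below it at the spawner's height.
; When debug drawing is enabled, Tick draws the spawn radius circle, spheres at both points and connecting lines, on authority only.
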(event EventTick
  (params (DeltaSeconds :type Float%20%28single-precision%29))
  (Networking|SwitchHasAuthority
    (:Authority
      (if (Variables|Debug|GetDebugDrawSpawnCircle)
        (Rendering|Debug|DrawDebugCircle (Transformation|GetActorLocation) (Variables|Default|GetAirSpawnRadius) 100 "(R=1.000000,G=0.047707,B=0.000000,A=1.000000)" 0.0 1e+02 "1.000000,0.000000,0.000000" "0.000000,1.000000,0.000000")
        (for _index (range 0 (- (Utilities|Array|Length (Variables|Default|GetDropZoneLocations)) 1))
          (Rendering|Debug|DrawDebugSphere (Utilities|Array|Get(acopy) (Variables|Default|GetDropZoneLocations) _index) 1.5e+02 12 "(R=0.000000,G=0.277276,B=1.000000,A=1.000000)" 0.0 1e+01)
          (Rendering|Debug|DrawDebugSphere (Utilities|Array|Get(acopy) (Variables|Default|GetAirDropLocations) _index) 1.5e+02 12 "(R=0.000000,G=0.277276,B=1.000000,A=1.000000)" 0.0 1e+01)
          (Rendering|Debug|DrawDebugLine (Utilities|Array|Get(acopy) (Variables|Default|GetDropZoneLocations) _index) (Utilities|Array|Get(acopy) (Variables|Default|GetAirDropLocations) _index) "(R=1.000000,G=0.000000,B=0.012991,A=1.000000)" 0.0 1e+01))))))

(event EventSetDebugLocations
  (for _array_element (Variables|Default|GetItemDropZones)
    (Utilities|Array|Add (Variables|Default|GetDropZoneLocations) (Transformation|GetActorLocation _array_element))
    (Utilities|Array|Add (Variables|Default|GetAirDropLocations) (Math|Vector|MakeVector (.x (Transformation|GetActorLocation _array_element)) (.y (Transformation|GetActorLocation _array_element)) (.z (Transformation|GetActorLocation))))))

(fn ConstructionScript)