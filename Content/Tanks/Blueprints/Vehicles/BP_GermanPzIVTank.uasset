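; Panzer IV tank Blueprint that is driven by an AI behavior tree.
; On BeginPlay, only the network authority tells the tank's AI controller to run BT_Tank.
; Tick stores the mesh's velocity magnitude as the current speed.
; FindTargetLocation gathers the unique locations of all TargetPoint actors into TargetLocations, but nothing in this file calls it.
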(event EventTick
  (params (DeltaSeconds :type Float%20%28single-precision%29))
  (Variables|Default|SetCurretSpeed (Math|Vector|VectorLength (Transformation|GetComponentVelocity (Variables|Character|GetMesh)))))

(event EventBeginPlay
  (Networking|SwitchHasAuthority
    (:Authority
      (AI|RunBehaviorTree (AI|GetAIController self) "/Game/Tanks/AI/BehaviorTree/BT_Tank.BT_Tank"))))

(fn ConstructionScript)

(fn FindTargetLocation
  (bind _outactors (Actor|GetAllActorsOfClass "/Script/Engine.TargetPoint"))
  (for _array_element _outactors
    (Utilities|Array|AddUnique (Variables|Default|GetTargetLocations) (Transformation|GetActorLocation _array_element))))