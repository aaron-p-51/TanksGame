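; Player tank vehicle Blueprint with helper functions for rollover recovery and engine exhaust effects.
; CanFlipOver reports when absolute roll or pitch reaches a tilt threshold.
; Flip launches the mesh upward with a mass-independent impulse and lowers its center of mass, with no reset in these graphs.
; SetExhaustSmoke scales the spawn rate of two smoke effects with engine rotation speed relative to its maximum.
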(fn ConstructionScript)

(fn CanFlipOver
  (bind _returnvalue (Transformation|GetActorRotation))
  (return (or (>= (Math|Float|Absolute(Float) (.roll _returnvalue)) 3e+01) (>= (Math|Float|Absolute(Float) (.pitch _returnvalue)) 3e+01))))

(fn Flip
  (bind _mesh (Variables|Character|GetMesh))
  (Physics|AddImpulse _mesh "0, 0,500.000000" "None" true)
  (Class|PrimitiveComponent|SetCenterOfMass _mesh "0, 0,-100.000000" "None"))

(fn SetExhaustSmoke
  (bind _vehiclemovement (Variables|Default|GetVehicleMovement))
  (bind _returnvalue (Class|WheeledVehicleMovementComponent|GetEngineMaxRotationSpeed _vehiclemovement))
  (bind _returnvalue_2 (Class|WheeledVehicleMovementComponent|GetEngineRotationSpeed _vehiclemovement))
  (bind _returnvalue_3 (Math|Float|MapRangeClamped _returnvalue_2 0.0 _returnvalue 5e+01 2e+02))
  (Utilities|FlowControl|Sequence
    (:then_0
      (Niagara|SetNiagaraVariable(Float) (Variables|Default|GetTempSmoke) "SpawnRate" _returnvalue_3))
    (:then_1
      (Niagara|SetNiagaraVariable(Float) (Variables|Default|GetTempSmoke1) "SpawnRate" _returnvalue_3))))