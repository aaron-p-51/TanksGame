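; BP_TestLineTraceCollision is a dev-testing actor that checks which physical material a line trace hits.
; On BeginPlay, a looping one-second timer fires a Visibility-channel trace forward from the LineTraceStart component, with debug drawing.
; Each hit prints the display name of the physical material it struck.
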(event Custom|DoLineTrace
  (bind _linetracestart (Variables|Default|GetLineTraceStart))
  (bind _returnvalue (Transformation|GetWorldLocation _linetracestart))
  (bind (_outhit _returnvalue_2) (Collision|LineTraceByChannel _returnvalue (+ _returnvalue (* (Math|Vector|GetForwardVector (Transformation|GetWorldRotation _linetracestart)) 1e+03)) "TraceTypeQuery1" false 0 "ForDuration"))
  (if _returnvalue_2
    (Development|PrintString (Utilities|GetDisplayName (.PhysMat (Collision|BreakHitResult _outhit))))))

(event EventBeginPlay
  (Utilities|Time|SetTimerbyEvent (delegate Custom|DoLineTrace) 1.0 true))

(event Collision|EventActorBeginOverlap
  (params (OtherActor :type Actor%20Object%20Reference)))

(event EventTick
  (params (DeltaSeconds :type Float%20%28single-precision%29)))

(fn ConstructionScript)