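; Behavior tree service for tank AI that selects the closest sensed actor as the combat target.
; On each tick it loops over the AI perception component's perceived actors, comparing squared distances to the controlled pawn, with no filter for players.
; The result, or None if nothing qualifies, goes to a blackboard key and to CurrentCombatTarget on the TBaseAIController.
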(event EventReceiveTickAI
  (params (OwnerController :type AI%20Controller%20Object%20Reference) (ControlledPawn :type Pawn%20Object%20Reference) (DeltaSeconds :type Float%20%28single-precision%29))
  ;[1 1 1] Set Initial values, Get Known actors
  (Variables|Default|SetBestTargetActor 0)
  (Variables|Default|SetDistanceToClosestTarget 1e+09)
  (for _array_element (Class|AIPerceptionComponent|GetPerceivedActors (Actor|GetComponentbyClass OwnerController "/Script/AIModule.AIPerceptionComponent"))
    (if (< (Math|Vector|VectorLengthSquared (- (Transformation|GetActorLocation ControlledPawn) (Transformation|GetActorLocation _array_element))) (Variables|Default|GetDistanceToClosestTarget))
      (Variables|Default|SetDistanceToClosestTarget (Math|Vector|VectorLengthSquared (- (Transformation|GetActorLocation ControlledPawn) (Transformation|GetActorLocation _array_element))))
      (Variables|Default|SetBestTargetActor _array_element)))
  (Class|BTFunctionLibrary|SetBlackboardValueasObject (Variables|Default|GetBlackBoardKey) (Variables|Default|GetBestTargetActor))
  (bind _astbase_aicontroller (Utilities|Casting|CastToTBaseAIController OwnerController))
  (Variables|/Script/Tanks.TBaseAIController|SetCurrentCombatTarget _astbase_aicontroller (Variables|Default|GetBestTargetActor)))