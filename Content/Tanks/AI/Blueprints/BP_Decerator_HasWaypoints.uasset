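; Behavior tree decorator for tank AI that passes only when the controlled pawn has valid waypoints.
; It finds the pawn's TWaypointsComponent, caches the reference and returns the result of its HasValidWaypoints check.
; If no component is found it prints an "Invalid Waypoint" debug message.
; An unconnected older variant that casts to BP_EnemyTankBase remains in the graph but never runs.
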(fn PerformConditionCheckAI
  (params (OwnerController :type AI%20Controller%20Object%20Reference) (ControlledPawn :type Pawn%20Object%20Reference))
  (Utilities|IsValid (LocalVariables|GetWaypointCompRef)
    (:Is%20Valid
      _)
    (:Is%20Not%20Valid
      (LocalVariables|SetWaypointCompRef (Actor|GetComponentbyClass ControlledPawn "/Script/Tanks.TWaypointsComponent"))))
  (Utilities|IsValid (LocalVariables|GetWaypointCompRef)
    (:Is%20Valid
      (bind _returnvalue (Class|TWaypointsComponent|HasValidWaypoints (LocalVariables|GetWaypointCompRef)))
      (return _returnvalue))
    (:Is%20Not%20Valid
      (Development|PrintString "Invalid Waypoint"))))