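; Behavior tree task for tank AI that fires the controlled pawn's weapon for a timed burst.
; It sends start and stop fire messages through the shootable weapon owner interface around a delay, then succeeds; pawns lacking the interface never finish it.
; ComputeFireDuration supplies the delay, but its randomized deviation math is unconnected.
; The branch setting the controller's combat target from the blackboard never runs.
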(event EventReceiveExecuteAI
  (params (OwnerController :type AI%20Controller%20Object%20Reference) (ControlledPawn :type Pawn%20Object%20Reference))
  (if (Utilities|DoesObjectImplementInterface ControlledPawn "/Script/Tanks.TShootableWeaponOwner")
    (Class|TShootableWeaponOwner|StartFire(Message) ControlledPawn)
    (Utilities|FlowControl|Delay (Utilities|ComputeFireDuration (Variables|WeaponFire|GetFireDeviation) (Variables|WeaponFire|GetFireDuration)))
    (Class|TShootableWeaponOwner|StopFire(Message) ControlledPawn)
    (AI|BehaviorTree|FinishExecute true)))