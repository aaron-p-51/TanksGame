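; Behavior tree task that moves the AI-controlled pawn to a blackboard location at a set walk speed.
; On execute it writes MoveToSpeed, clamped to be non-negative, into the pawn's CharacterMovementComponent, then runs AI MoveTo toward the MoveToLocation key's vector.
; The move result finishes the task as success or failure, and a pawn without that movement component aborts it.
; The previous walk speed is not restored afterward.
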(event EventReceiveExecuteAI
  (params (OwnerController :type AI%20Controller%20Object%20Reference) (ControlledPawn :type Pawn%20Object%20Reference))
  (bind _returnvalue (Actor|GetComponentbyClass ControlledPawn "/Script/Engine.CharacterMovementComponent"))
  (Utilities|IsValid _returnvalue
    (:Is%20Valid
      (Variables|/Script/Engine.CharacterMovementComponent|SetMaxWalkSpeed _returnvalue (Math|Float|Clamp(Float) (Variables|Default|GetMoveToSpeed) 0.0 9999999.0))
      (AI|AIMoveTo ControlledPawn (Class|BTFunctionLibrary|GetBlackboardValueasVector (Variables|Default|GetMoveToLocation)) 0 5.0 false
        (:OnSuccess
          (AI|BehaviorTree|FinishExecute true))
        (:OnFail
          (AI|BehaviorTree|FinishExecute false))))
    (:Is%20Not%20Valid
      (Class|BTTaskBlueprintBase|FinishAbort))))