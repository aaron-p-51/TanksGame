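; Behavior tree decorator for tank AI that passes when the blackboard target is further away than a set distance.
; It reads the Target actor from the blackboard and compares the squared distance from the controlled pawn against Distance squared, avoiding a square root.
; The check fails when no valid target is set.
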(fn PerformConditionCheckAI
  (params (OwnerController :type AI%20Controller%20Object%20Reference) (ControlledPawn :type Pawn%20Object%20Reference))
  (bind _distance (Variables|Default|GetDistance))
  (bind _target (Variables|Default|GetTarget))
  (bind _returnvalue (AI|BehaviorTree|GetBlackboardValueasActor _target))
  (Utilities|IsValid _returnvalue
    (:Is%20Valid
      (return (> (Math|Vector|VectorLengthSquared (- (Transformation|GetActorLocation ControlledPawn) (Transformation|GetActorLocation _returnvalue))) (* _distance _distance))))
    (:Is%20Not%20Valid
      (return false))))