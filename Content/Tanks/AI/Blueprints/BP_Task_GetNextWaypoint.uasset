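; Behavior tree task that picks the next patrol waypoint for an AI-controlled tank and writes it to the blackboard.
; On execute it reads the pawn's TWaypointsComponent, taking either a random or the next sequential waypoint based on the GetRandomWaypoint flag.
; The location is stored as a vector in the NextWaypoint key, and the task fails if the pawn has no waypoints component.
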(event EventReceiveExecuteAI
  (params (OwnerController :type AI%20Controller%20Object%20Reference) (ControlledPawn :type Pawn%20Object%20Reference))
  (bind _returnvalue (Actor|GetComponentbyClass ControlledPawn "/Script/Tanks.TWaypointsComponent"))
  (bind _nextwaypoint (Variables|Default|GetNextWaypoint))
  (Utilities|IsValid _returnvalue
    (:Is%20Valid
      (if (Variables|Default|GetGetRandomWaypoint)
        (bind _returnvalue_2 (Class|TWaypointsComponent|GetRandomWaypoint _returnvalue))
        (AI|BehaviorTree|SetBlackboardValueasVector _nextwaypoint _returnvalue_2)
        (else
          (bind _returnvalue_3 (Class|TWaypointsComponent|GetNextWaypoint _returnvalue))
          (AI|BehaviorTree|SetBlackboardValueasVector _nextwaypoint _returnvalue_3)))
      (AI|BehaviorTree|FinishExecute true))
    (:Is%20Not%20Valid
      (AI|BehaviorTree|FinishExecute false))))