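; Enemy defense tower that tracks the player tank and fires team-tagged bullets at it in a demo tank game.
; A sphere overlap sets the target, and each Tick a validity macro drives the anim instance's aim blend, recoil and a frame-counted reload.
; Opposing bullets reduce life on mesh overlap; at zero it plays a death animation, sinks below the floor and destroys itself.
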(event OnComponentBeginOverlap(SkeletalMesh)
  (params (OverlappedComponent :type Primitive%20Component%20Object%20Reference) (OtherActor :type Actor%20Object%20Reference) (OtherComp :type Primitive%20Component%20Object%20Reference) (OtherBodyIndex :type Integer) (bFromSweep :type Boolean) (SweepResult :type Hit%20Result%20Structure%20%28by%20ref%29))
  ;[1 1 1] Detect hit
  (bind _asbp_bullet (Utilities|Casting|CastToBP_Bullet OtherActor))
  (if (Utilities|Enum|NotEqual(Enum) (Variables|/Game/SCTanks_OLD/DemoSimpleGame/BluePrints/BP_Bullet.BP_Bullet_C|GetTeam _asbp_bullet) (Variables|Default|GetTeam))
    (Actor|DestroyActor OtherActor)
    (Audio|PlaySoundatLocation "/Game/SCTanks_OLD/DemoSimpleGame/Sounds/shellExplosive.shellExplosive" (Transformation|GetActorLocation) "0, 0, 0" 0.4 1.0 0.0 "/Game/SCTanks_OLD/DemoSimpleGame/Sounds/NewSoundAttenuation.NewSoundAttenuation" 0 0)
    (if (> (Variables|Default|GetLifeStat) 0.0)
      (bind _output_get (Variables|Default|SetLifeStat (- (Variables|Default|GetLifeStat) 3e+01)))
      (if (not (> _output_get 0.0))
        (Components|Animation|PlayAnimation (Variables|Default|GetSkeletalMesh) "/Game/SCTanks_OLD/Animations/Anim_SCT_Tower_Dead.Anim_SCT_Tower_Dead" false)
        (Audio|PlaySoundatLocation "/Game/SCTanks_OLD/DemoSimpleGame/Sounds/unitDead.unitDead" (Transformation|GetWorldLocation (Variables|Default|GetSkeletalMesh)) "0, 0, 0" 0.4 1.0 0.0 "/Game/SCTanks_OLD/DemoSimpleGame/Sounds/NewSoundAttenuation.NewSoundAttenuation" 0 0)))))

(event OnComponentBeginOverlap(Sphere)
  (params (OverlappedComponent :type Primitive%20Component%20Object%20Reference) (OtherActor :type Actor%20Object%20Reference) (OtherComp :type Primitive%20Component%20Object%20Reference) (OtherBodyIndex :type Integer) (bFromSweep :type Boolean) (SweepResult :type Hit%20Result%20Structure%20%28by%20ref%29))
  ;[1 1 1] Detect terget
  (bind _asbp_tank_player (Utilities|Casting|CastToBP_TankPlayer OtherActor))
  (Variables|Default|Settarget _asbp_tank_player))

(event OnComponentEndOverlap(Sphere)
  (params (OverlappedComponent :type Primitive%20Component%20Object%20Reference) (OtherActor :type Actor%20Object%20Reference) (OtherComp :type Primitive%20Component%20Object%20Reference) (OtherBodyIndex :type Integer))
  ;[1 1 1] Remove Target
  (Utilities|Casting|CastToBP_TankPlayer OtherActor)
  (Variables|Default|Settarget 0))

(event EventTick
  (params (DeltaSeconds :type Float%20%28single-precision%29))
  (bind _returnvalue (Transformation|GetActorLocation))
  (bind _skeletalmesh (Variables|Default|GetSkeletalMesh))
  (bind _target (Variables|Default|Gettarget))
  (bind _returnvalue_2 (Transformation|GetSocketLocation _skeletalmesh "GunEndSocket"))
  (bind _returnvalue_3 (Transformation|GetActorLocation _target))
  (bind _returnvalue_4 (Math|Rotator|FindLookatRotation _returnvalue _returnvalue_3))
  (if (> (Variables|Default|GetLifeStat) 0.0)
    ;[1 1 1] if see target
    (|validTarget
      (:then
        (bind _asbp_tower_defense_animation (Utilities|Casting|CastToBP_TowerDefense_Animation (Components|SkeletalMesh|GetAnimInstance (Variables|Default|GetSkeletalMesh))))
        (Variables|/Game/SCTanks_OLD/DemoSimpleTactics/BluePrints/BP_TowerDefense_Animation.BP_TowerDefense_Animation_C|SetSt_DoBlend _asbp_tower_defense_animation true)
        (Variables|/Game/SCTanks_OLD/DemoSimpleTactics/BluePrints/BP_TowerDefense_Animation.BP_TowerDefense_Animation_C|SetSt_ToRotate _asbp_tower_defense_animation (Math|Rotator|MakeRotator 0.0 0.0 (+ (.Yaw (Math|Rotator|BreakRotator _returnvalue_4)) 9e+01)))
        (if (> (Variables|/Game/SCTanks_OLD/DemoSimpleTactics/BluePrints/BP_TowerDefense_Animation.BP_TowerDefense_Animation_C|GetST_BlendControlRotate _asbp_tower_defense_animation) 0.9)
          (if (== (Variables|Default|GetShotReload) 0)
            ;[1 1 1] Bullet
            (Variables|Default|SetShotReload 255)
            (Variables|/Game/SCTanks_OLD/DemoSimpleTactics/BluePrints/BP_TowerDefense_Animation.BP_TowerDefense_Animation_C|SetST_ShotRecoil _asbp_tower_defense_animation -15.0)
            (bind _returnvalue_5 (Game|SpawnActorfromClass "/Game/SCTanks_OLD/DemoSimpleGame/BluePrints/BP_Bullet.BP_Bullet_C" (Math|Transform|MakeTransform _returnvalue_2 _returnvalue_4 "0.500000,0.300000,0.300000") "Undefined" 0 0))
            (Variables|/Game/SCTanks_OLD/DemoSimpleGame/BluePrints/BP_Bullet.BP_Bullet_C|SetTeam _returnvalue_5 (Variables|Default|GetTeam))
            (Audio|PlaySoundatLocation "/Game/SCTanks_OLD/DemoSimpleGame/Sounds/tankShot.tankShot" _returnvalue_2 "0, 0, 0" 1.5 1.0 0.0 0 0 0)
            (else
              (Math|Integer|DecrementInt (Variables|Default|GetShotReload))))))
      (:OutputPin
        ;[1 1 1] Dont see target
        (bind _asbp_tower_defense_animation_2 (Utilities|Casting|CastToBP_TowerDefense_Animation (Components|SkeletalMesh|GetAnimInstance (Variables|Default|GetSkeletalMesh))))
        (Variables|/Game/SCTanks_OLD/DemoSimpleTactics/BluePrints/BP_TowerDefense_Animation.BP_TowerDefense_Animation_C|SetSt_DoBlend _asbp_tower_defense_animation_2 false)))
    (else
      ;[1 1 1] destroy
      (bind _output_get (Variables|Default|SetunderFloor (- (Variables|Default|GetunderFloor) 0.1)))
      (if (> _output_get -1e+02)
        (Transformation|SetRelativeTransform (Variables|Default|GetSkeletalMesh) (Math|Transform|MakeTransform (Math|Vector|MakeVector 0.0 0.0 _output_get) "0, 0, 0" "1,1,1") false false)
        (else
          (Actor|DestroyActor))))))

(fn ConstructionScript)