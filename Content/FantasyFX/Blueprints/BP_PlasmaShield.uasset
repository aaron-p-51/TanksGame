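; BP_PlasmaShield is a plasma shield effect actor with moving and non-moving variants, selected by the IsMoving flag.
; The construction script sets the shield material for the chosen variant and shows three gyro components only when it is not moving.
; Each tick aligns the Scene component along the line from the player camera, billboard-style, and spins the gyros at GyroSpeed in the non-moving variant.
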(event EventBeginPlay)

(event Collision|EventActorBeginOverlap
  (params (OtherActor :type Actor%20Object%20Reference)))

(event EventTick
  (params (DeltaSeconds :type Float%20%28single-precision%29))
  (bind _scene (Variables|Default|GetScene))
  (bind _gyrospeed (Variables|Default|GetGyroSpeed))
  (bind _returnvalue (* DeltaSeconds _gyrospeed))
  (Transformation|SetWorldRotation _scene (Math|Rotator|FindLookatRotation (Camera|GetCameraLocation (Game|GetPlayerCameraManager 0)) (Transformation|GetWorldLocation _scene)) false false)
  ;[1 1 1] Gyro
  (if (not (Variables|Default|GetIsMoving?))
    (Transformation|AddLocalRotation (Variables|Default|GetGyro) (Math|Rotator|MakeRotator _returnvalue _returnvalue _returnvalue) false false)))

(fn ConstructionScript
  (bind _shield (Variables|Default|GetShield))
  (bind _gyro2 (Variables|Default|GetGyro2))
  (if (Variables|Default|GetIsMoving?)
    (Rendering|Material|SetMaterial _shield 0 "/Game/FantasyFX/Materials/Plasma/M_Plasma_Shield.M_Plasma_Shield")
    (Rendering|SetVisibility _gyro2 false false)
    (else
      (Rendering|Material|SetMaterial _shield 0 "/Game/FantasyFX/Materials/Plasma/M_Plasma_Shield_NotMoving.M_Plasma_Shield_NotMoving")
      (Rendering|SetVisibility _gyro2 true false))))