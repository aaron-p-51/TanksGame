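; Nature projectile spawner that, while IsActive is set, repeatedly fires volleys of five BP_Nature_Projectile actors.
; Tick feeds a DoOnce into staggered delayed branches, each spawning at Arrow's location with one of five arrow rotations.
; PSplashSpawn is switched on before each shot and off afterward; nodes that would rotate it are unwired.
; The DoOnce resets after a cooldown following the last shot, or whenever IsActive is false.
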(event EventBeginPlay)

(event EventTick
  (params (DeltaSeconds :type Float%20%28single-precision%29))
  (if (Variables|Default|GetIsActive) :!label _label
    (Utilities|FlowControl|DoOnce false :!label _label_2
      (:Completed
        (Utilities|FlowControl|Delay 1.0)
        (Utilities|FlowControl|Sequence
          (:then_0
            (Components|Activation|SetActive (Variables|Default|GetP_Splash_Spawn) true false)
            (Utilities|FlowControl|Delay 0.2)
            (Game|SpawnActorfromClass "/Game/FantasyFX/Blueprints/BP_Nature_Projectile.BP_Nature_Projectile_C" (Math|Transform|MakeTransform (Transformation|GetWorldLocation (Variables|Default|GetArrow)) (Transformation|GetWorldRotation (Variables|Default|GetArrow1)) "1,1,1") "AlwaysSpawn" 0 0)
            (Components|Activation|SetActive (Variables|Default|GetP_Splash_Spawn) false false))
          (:then_1
            (Utilities|FlowControl|Delay 0.1)
            (Components|Activation|SetActive (Variables|Default|GetP_Splash_Spawn) true false)
            (Utilities|FlowControl|Delay 0.2)
            (Game|SpawnActorfromClass "/Game/FantasyFX/Blueprints/BP_Nature_Projectile.BP_Nature_Projectile_C" (Math|Transform|MakeTransform (Transformation|GetWorldLocation (Variables|Default|GetArrow)) (Transformation|GetWorldRotation (Variables|Default|GetArrow2)) "1,1,1") "AlwaysSpawn" 0 0)
            (Components|Activation|SetActive (Variables|Default|GetP_Splash_Spawn) false false))
          (:then_2
            (Utilities|FlowControl|Delay 0.2)
            (Components|Activation|SetActive (Variables|Default|GetP_Splash_Spawn) true false)
            (Utilities|FlowControl|Delay 0.2)
            (Game|SpawnActorfromClass "/Game/FantasyFX/Blueprints/BP_Nature_Projectile.BP_Nature_Projectile_C" (Math|Transform|MakeTransform (Transformation|GetWorldLocation (Variables|Default|GetArrow)) (Transformation|GetWorldRotation (Variables|Default|GetArrow3)) "1,1,1") "AlwaysSpawn" 0 0)
            (Components|Activation|SetActive (Variables|Default|GetP_Splash_Spawn) false false))
          (:then_3
            (Utilities|FlowControl|Delay 0.3)
            (Components|Activation|SetActive (Variables|Default|GetP_Splash_Spawn) true false)
            (Utilities|FlowControl|Delay 0.2)
            (Game|SpawnActorfromClass "/Game/FantasyFX/Blueprints/BP_Nature_Projectile.BP_Nature_Projectile_C" (Math|Transform|MakeTransform (Transformation|GetWorldLocation (Variables|Default|GetArrow)) (Transformation|GetWorldRotation (Variables|Default|GetArrow4)) "1,1,1") "AlwaysSpawn" 0 0)
            (Components|Activation|SetActive (Variables|Default|GetP_Splash_Spawn) false false))
          (:then_4
            (Utilities|FlowControl|Delay 0.4)
            (Components|Activation|SetActive (Variables|Default|GetP_Splash_Spawn) true false)
            (Utilities|FlowControl|Delay 0.2)
            (Game|SpawnActorfromClass "/Game/FantasyFX/Blueprints/BP_Nature_Projectile.BP_Nature_Projectile_C" (Math|Transform|MakeTransform (Transformation|GetWorldLocation (Variables|Default|GetArrow)) (Transformation|GetWorldRotation (Variables|Default|GetArrow5)) "1,1,1") "AlwaysSpawn" 0 0)
            (Components|Activation|SetActive (Variables|Default|GetP_Splash_Spawn) false false)
            (Utilities|FlowControl|Delay 3.0)
            (Utilities|FlowControl|Sequence
              (:then_0
                (goto _label))
              (:then_1
                (goto _label_2 Reset)))))))
    (else
      (goto _label_2 Reset))))

(fn ConstructionScript)