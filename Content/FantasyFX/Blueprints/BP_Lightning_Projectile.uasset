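; BP_Lightning_Projectile is a FantasyFX lightning projectile that bursts into an impact effect when its collision component hits something.
; A DoOnce limits the response to the first hit, which spawns the P_Lightning_Impact emitter slightly offset along world Y, then destroys the actor.
; Cross products with the impact normal set the emitter's roll and yaw, while randomized pitch and per-axis scale vary each impact.
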(event OnComponentHit(Collision)
  (params (HitComponent :type Primitive%20Component%20Object%20Reference) (OtherActor :type Actor%20Object%20Reference) (OtherComp :type Primitive%20Component%20Object%20Reference) (NormalImpulse :type Vector :default "0, 0, 0") (Hit :type Hit%20Result%20Structure%20%28by%20ref%29))
  (bind _returnvalue (Math|Vector|MakeVector 0.0 0.0 1.0))
  (bind (_bblockinghit _binitialoverlap _time _location _impactpoint _normal _impactnormal) (Collision|BreakHitResult Hit))
  (bind _returnvalue_2 (Math|Random|RandomFloatinRange 1.5 2.5))
  (bind _returnvalue_3 (Math|Vector|CrossProduct _returnvalue _impactnormal))
  (bind (_x _y _z) (Math|Vector|BreakVector _location))
  (bind _returnvalue_4 (Math|Vector|CrossProduct _returnvalue_3 _impactnormal))
  (bind _returnvalue_5 (Math|Rotator|MakeRotationfromAxes _returnvalue_4 _returnvalue_3 _impactnormal))
  (bind (_roll _pitch _yaw) (Math|Rotator|BreakRotator _returnvalue_5))
  (Utilities|FlowControl|DoOnce false
    (:Completed
      (bind _returnvalue_6 (Effects|SpawnEmitteratLocation "/Game/FantasyFX/Particles/Lightning/P_Lightning_Impact.P_Lightning_Impact" (Math|Vector|MakeVector (+ _x 0.0) (+ _y 15.0) _z) (Math|Rotator|MakeRotator (- _roll 9e+01) (Math|Random|RandomFloatinRange 0.0 3.6e+02) (+ _yaw 9e+01))))
      (Transformation|SetWorldScale3D _returnvalue_6 (Math|Vector|MakeVector _returnvalue_2 _returnvalue_2 _returnvalue_2))
      (Actor|DestroyActor))))

(event EventBeginPlay)

(fn ConstructionScript)